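; Battery pickup actor that adds one to the ThirdPersonCharacter's BatteryCapacity.
; A box overlap sets a flag for any overlapping actor, and Tick polls for any held key while that flag is set.
; Below the capacity cap it increments the count and destroys itself; otherwise it prints that no more can be carried.
; Overlap changes also print debug messages.
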(event OnComponentBeginOverlap(Box)
  (params (OverlappedComponent :type Primitive%20Component%20Object%20Reference) (OtherActor :type Actor%20Object%20Reference) (OtherComp :type Primitive%20Component%20Object%20Reference) (OtherBodyIndex :type Integer) (bFromSweep :type Boolean) (SweepResult :type Hit%20Result%20Structure%20%28by%20ref%29))
  (Variables|Default|Setoverlapping true)
  (Development|PrintString "colision"))

(event OnComponentEndOverlap(Box)
  (params (OverlappedComponent :type Primitive%20Component%20Object%20Reference) (OtherActor :type Actor%20Object%20Reference) (OtherComp :type Primitive%20Component%20Object%20Reference) (OtherBodyIndex :type Integer))
  (Variables|Default|Setoverlapping false)
  (Development|PrintString "no colision"))

(event EventTick
  (params (DeltaSeconds :type Float%20%28single-precision%29))
  (Utilities|FlowControl|Sequence
    (:then_0
      (if (Variables|Default|Getoverlapping)
        (if (Game|Player|IsInputKeyDown (Game|GetPlayerController 0) "AnyKey")
          (bind _asthird_person_character (Utilities|Casting|CastToThirdPersonCharacter (Game|GetPlayerCharacter 0)))
          (if (< (Variables|/Game/ThirdPersonBP/Blueprints/ThirdPersonCharacter.ThirdPersonCharacter_C|GetBattery%20Capacity _asthird_person_character) 5)
            (Variables|/Game/ThirdPersonBP/Blueprints/ThirdPersonCharacter.ThirdPersonCharacter_C|SetBattery%20Capacity _asthird_person_character (+ (Variables|/Game/ThirdPersonBP/Blueprints/ThirdPersonCharacter.ThirdPersonCharacter_C|GetBattery%20Capacity _asthird_person_character) 1))
            (Actor|DestroyActor)
            (else
              (Development|PrintString "no puede cargar mas"))))))))

(fn ConstructionScript)