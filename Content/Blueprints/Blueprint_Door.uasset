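; Door actor that opens and closes on demand while something overlaps its Caja trigger component.
; Begin and end overlap set a Collision flag, with no filter on the overlapping actor, and the abrirPuerta event acts only while that flag is set.
; A FlipFlop alternates each accepted call between setting PlayerNear true and false on the skeletal mesh's puerta animation instance, which presumably drives the door animation.
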(event OnComponentBeginOverlap(caja)
  (params (OverlappedComponent :type Primitive%20Component%20Object%20Reference) (OtherActor :type Actor%20Object%20Reference) (OtherComp :type Primitive%20Component%20Object%20Reference) (OtherBodyIndex :type Integer) (bFromSweep :type Boolean) (SweepResult :type Hit%20Result%20Structure%20%28by%20ref%29))
  (Variables|Default|Setcollision true))

(event OnComponentEndOverlap(caja)
  (params (OverlappedComponent :type Primitive%20Component%20Object%20Reference) (OtherActor :type Actor%20Object%20Reference) (OtherComp :type Primitive%20Component%20Object%20Reference) (OtherBodyIndex :type Integer))
  (Variables|Default|Setcollision false))

(event Custom|abrirPuerta
  (if (Variables|Default|Getcollision)
    (Utilities|FlowControl|FlipFlop
      (:A
        (bind _aspuerta (Utilities|Casting|CastTopuerta (Components|SkeletalMesh|GetAnimInstance (Variables|Default|GetSkeletalMesh))))
        (Variables|/Game/Horror_pack/Animation/Door/puerta.puerta_C|SetplayerNear _aspuerta true))
      (:B
        (bind _aspuerta_2 (Utilities|Casting|CastTopuerta (Components|SkeletalMesh|GetAnimInstance (Variables|Default|GetSkeletalMesh))))
        (Variables|/Game/Horror_pack/Animation/Door/puerta.puerta_C|SetplayerNear _aspuerta_2 false)))))

(event EventBeginPlay
  (Variables|Default|Setcollision false))

(fn ConstructionScript)